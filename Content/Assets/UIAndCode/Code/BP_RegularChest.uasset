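; BP_RegularChest is an interactable chest that opens when it receives a BPIInteract call.
; It creates an InteractPrompt widget on BeginPlay and shows or hides it as the player character enters or leaves the Box trigger.
; Interaction switches on EnumStatus: a closed chest becomes Open with an animation and sound.
; An open chest only resets its status to Closed, with no closing animation or sound.
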(event OnComponentBeginOverlap(Box)
  (params (OverlappedComponent :type Primitive%20Component%20Object%20Reference) (OtherActor :type Actor%20Object%20Reference) (OtherComp :type Primitive%20Component%20Object%20Reference) (OtherBodyIndex :type Integer) (bFromSweep :type Boolean) (SweepResult :type Hit%20Result%20Structure%20%28by%20ref%29))
  (if (== OtherActor (Game|GetPlayerCharacter 0))
    (UserInterface|Viewport|AddtoViewport (stale EventBeginPlay _returnvalue) 0)))

(event OnComponentEndOverlap(Box)
  (params (OverlappedComponent :type Primitive%20Component%20Object%20Reference) (OtherActor :type Actor%20Object%20Reference) (OtherComp :type Primitive%20Component%20Object%20Reference) (OtherBodyIndex :type Integer))
  (if (== OtherActor (Game|GetPlayerCharacter 0))
    (Widget|RemovefromParent (stale EventBeginPlay _returnvalue))))

(event EventBeginPlay
  (bind _returnvalue (UserInterface|CreateWidget "/Game/Assets/UIAndCode/UI/InteractPrompt.InteractPrompt_C")))

(event Collision|EventActorBeginOverlap
  (params (OtherActor :type Actor%20Object%20Reference)))

(event EventTick
  (params (DeltaSeconds :type Float%20%28single-precision%29)))

(event EventBPIInteract
  (switch Utilities|FlowControl|Switch|SwitchonEnum_Status (Variables|Default|GetEnum_Status)
    (:NewEnumerator0
      (Variables|Default|SetEnum_Status "NewEnumerator1")
      (Components|Animation|PlayAnimation (Variables|Default|GetRegularChest) "/Game/Assets/Mimic/RegularChest/RegularChest_Anim_ChestOpen.RegularChest_Anim_ChestOpen" false)
      (Audio|PlaySound2D "/Game/Assets/Audio/ChestOpenning.ChestOpenning" 1.0 1.0 0.0 0 0))
    (:NewEnumerator1
      (Variables|Default|SetEnum_Status "NewEnumerator0"))))

(fn ConstructionScript)