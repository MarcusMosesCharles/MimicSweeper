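; BP_Pseudo_Mimic is an interactable mimic actor that toggles between Closed and Open.
; A box overlap shows or hides an interact prompt widget for the player character.
; The BPIInteract event flips the status; opening also adds an audio component, sets MimicTriggered and, after a fixed delay, sets DelaySinceTriggered.
; Closing only resets the status, leaving both trigger flags set, and nothing in this graph reads those flags.
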(event OnComponentBeginOverlap(Box)
  (params (OverlappedComponent :type Primitive%20Component%20Object%20Reference) (OtherActor :type Actor%20Object%20Reference) (OtherComp :type Primitive%20Component%20Object%20Reference) (OtherBodyIndex :type Integer) (bFromSweep :type Boolean) (SweepResult :type Hit%20Result%20Structure%20%28by%20ref%29))
  (if (== OtherActor (Game|GetPlayerCharacter 0))
    (UserInterface|Viewport|AddtoViewport (Variables|Default|GetInteract%20Prompt) 0)))

(event OnComponentEndOverlap(Box)
  (params (OverlappedComponent :type Primitive%20Component%20Object%20Reference) (OtherActor :type Actor%20Object%20Reference) (OtherComp :type Primitive%20Component%20Object%20Reference) (OtherBodyIndex :type Integer))
  (if (== OtherActor (Game|GetPlayerCharacter 0))
    (Widget|RemovefromParent (Variables|Default|GetInteract%20Prompt))))

(event EventBeginPlay
  (bind _returnvalue (UserInterface|CreateWidget "/Game/Assets/UIAndCode/UI/InteractPrompt.InteractPrompt_C"))
  (Variables|Default|SetInteract%20Prompt _returnvalue)
  (Input|EnableInput (Game|GetPlayerController 0)))

(event EventBPIInteract
  (switch Utilities|FlowControl|Switch|SwitchonEnum_Status (Variables|Default|GetEnum_Status)
    (:NewEnumerator0
      (Variables|Default|SetEnum_Status "NewEnumerator1")
      (AddComponent|AddAudioComponent false)
      (Variables|Default|SetMimicTriggered true)
      (Utilities|FlowControl|Delay 4.2)
      (Variables|Default|SetDelaySinceTriggered true))
    (:NewEnumerator1
      (Variables|Default|SetEnum_Status "NewEnumerator0"))))

(fn ConstructionScript)