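; BP_Mimic2 is a mimic enemy that sits at an item spot until interacted with, then wakes and hunts the player.
; Interacting sets animation flags and chase mode, frees its item spot, then after a delay enables capsule collision and flags detection on the AI blackboard.
; Trigger overlaps track the player and attack range, while a DamagePlayerServer-to-DamagePlayerClient event pair subtracts player health.
; Its capsule ignores InteractableEntity-tagged actors when moving.
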(event OnComponentBeginOverlap(AttackTrigger)
  (params (OverlappedComponent :type Primitive%20Component%20Object%20Reference) (OtherActor :type Actor%20Object%20Reference) (OtherComp :type Primitive%20Component%20Object%20Reference) (OtherBodyIndex :type Integer) (bFromSweep :type Boolean) (SweepResult :type Hit%20Result%20Structure%20%28by%20ref%29))
  (bind _asbp_third_person_character (Utilities|Casting|CastToBP_ThirdPersonCharacter OtherActor))
  (Variables|Default|SetPlayerInRange true))

(event OnComponentEndOverlap(AttackTrigger)
  (params (OverlappedComponent :type Primitive%20Component%20Object%20Reference) (OtherActor :type Actor%20Object%20Reference) (OtherComp :type Primitive%20Component%20Object%20Reference) (OtherBodyIndex :type Integer))
  (Utilities|Casting|CastToBP_ThirdPersonCharacter OtherActor)
  (Variables|Default|SetPlayerInRange false))

(event OnComponentBeginOverlap(IdleDetectionRange)
  (params (OverlappedComponent :type Primitive%20Component%20Object%20Reference) (OtherActor :type Actor%20Object%20Reference) (OtherComp :type Primitive%20Component%20Object%20Reference) (OtherBodyIndex :type Integer) (bFromSweep :type Boolean) (SweepResult :type Hit%20Result%20Structure%20%28by%20ref%29))
  (bind _asbp_third_person_character (Utilities|Casting|CastToBP_ThirdPersonCharacter OtherActor))
  (Variables|Default|SetPlayer _asbp_third_person_character))

(event Custom|DamagePlayerClient
  (bind _asbp_third_person_character (Utilities|Casting|CastToBP_ThirdPersonCharacter (stale OnComponentBeginOverlap(AttackTrigger) _asbp_third_person_character)))
  (Variables|/Game/ThirdPerson/Blueprints/BP_ThirdPersonCharacter.BP_ThirdPersonCharacter_C|SetHealth _asbp_third_person_character (- (Variables|/Game/ThirdPerson/Blueprints/BP_ThirdPersonCharacter.BP_ThirdPersonCharacter_C|GetHealth _asbp_third_person_character) 2e+01)))

(event Custom|DamagePlayerServer
  (CallFunction|DamagePlayerClient))

(event EventInteract
  (params (InteractedWith :type Boolean))
  (CallFunction|PlayerDetection)
  (Utilities|FlowControl|Delay 3.1)
  (Collision|SetCollisionEnabled (Variables|Collision|GetCapsuleComponent) "QueryAndPhysics")
  (bind _asabp_mimic_2 (Utilities|Casting|CastToABP_Mimic2 (Components|SkeletalMesh|GetAnimInstance (Variables|Character|GetMesh))))
  (Variables|/Game/Content/Character/Mimic/Mimic_2/Animation/ABP_Mimic2.ABP_Mimic2_C|SetABP_Activated _asabp_mimic_2 true)
  (AI|Components|Blackboard|SetValueasBool (AI|GetBlackboard (AI|GetAIController self)) (Utilities|Name|MakeLiteralName "BB_PlayerDetected") true))

(event EventBeginPlay
  (bind _outactors (Actor|GetAllActorswithTag "InteractableEntity"))
  (for _array_element _outactors
    (Collision|IgnoreActorwhenMoving (Variables|Collision|GetCapsuleComponent) _array_element true)))

(fn ConstructionScript)

(fn PlayerDetection
  (bind _asabp_mimic_2 (Utilities|Casting|CastToABP_Mimic2 (Components|SkeletalMesh|GetAnimInstance (Variables|Character|GetMesh))))
  (Variables|/Game/Content/Character/Mimic/Mimic_2/Animation/ABP_Mimic2.ABP_Mimic2_C|SetPlayerInteractedWith _asabp_mimic_2 true)
  (Variables|/Game/Content/Character/Mimic/Mimic_2/Animation/ABP_Mimic2.ABP_Mimic2_C|SetActiveAndDeactive _asabp_mimic_2 1e+02)
  (Variables|Default|SetChaseMode true)
  (bind _asbp_item_spots (Utilities|Casting|CastToBP_ItemSpots (Variables|Default|GetCurrentItemSpot)))
  (Variables|/Game/Content/Scripts/BP_ItemSpots.BP_ItemSpots_C|SetUnocupiedSpot _asbp_item_spots true))